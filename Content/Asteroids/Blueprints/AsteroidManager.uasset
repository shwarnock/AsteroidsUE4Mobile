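; Asteroid manager for an Asteroids game that spawns, moves and splits asteroids.
; After a short delay at BeginPlay, it spawns large asteroids just outside random screen edges by deprojecting screen positions to world space.
; Each Tick moves them along their vectors and calls an off-screen relocation update.
; Flagged asteroids are destroyed, with large and medium ones spawning smaller pieces in random directions at the same position.
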(event EventBeginPlay
  (Utilities|FlowControl|Delay 3.0)
  (for _index (range 0 4)
    (bind _output_get (Variables|Default|SetStartSide (Utilities|Enum|ByteToEnumStartSide (Math|Conversions|ToByte(Integer) (Math|Random|RandomInteger 3)))))
    (bind _startpos (CallFunction|GetStartPos _output_get))
    (bind _createdasteroid (CallFunction|CreateAsteroid "NewEnumerator0" "0, 0, 0" _startpos))
    (Utilities|Array|Add (Variables|Default|GetAsteroids) _createdasteroid)))

(event EventTick
  (params (DeltaSeconds :type Float%20%28single-precision%29))
  (CallFunction|UpdateMovement DeltaSeconds)
  (CallFunction|CheckforDestroyedAsteroids))

(fn ConstructionScript)

(fn GetStartPos
  (params (StartSide :type StartSide%20Enum :default "NewEnumerator0"))
  (bind _returnvalue (Game|GetPlayerController 0))
  (bind (_sizex _sizey) (HUD|GetViewportSize _returnvalue))
  (bind _returnvalue_2 (Math|Random|RandomInteger _sizex))
  (bind _returnvalue_3 (Math|Random|RandomInteger _sizey))
  (bind _returnvalue_4 (Math|Conversions|ToFloat(Integer) _returnvalue_2))
  (bind _returnvalue_5 (Math|Conversions|ToFloat(Integer) _returnvalue_3))
  (switch Utilities|FlowControl|Switch|SwitchonStartSide StartSide
    (:NewEnumerator0
      (return (.WorldPosition (Class|GameplayStatics|DeprojectScreentoWorld _returnvalue (Math|Vector2D|MakeVector2D -5e+01 _returnvalue_5)))))
    (:NewEnumerator1
      (return (.WorldPosition (Class|GameplayStatics|DeprojectScreentoWorld _returnvalue (Math|Vector2D|MakeVector2D (Math|Conversions|ToFloat(Integer) (+ _sizex 40)) _returnvalue_5)))))
    (:NewEnumerator2
      (return (.WorldPosition (Class|GameplayStatics|DeprojectScreentoWorld _returnvalue (Math|Vector2D|MakeVector2D _returnvalue_4 -5e+01)))))
    (:NewEnumerator3
      (return (.WorldPosition (Class|GameplayStatics|DeprojectScreentoWorld _returnvalue (Math|Vector2D|MakeVector2D _returnvalue_4 (Math|Conversions|ToFloat(Integer) (+ _sizey 40)))))))))

(fn UpdateMovement
  (params (DeltaTime :type Float%20%28single-precision%29))
  (for _array_element (Variables|Default|GetAsteroids)
    (Utilities|IsValid _array_element
      (:Is%20Valid
        (Transformation|SetActorLocation _array_element (+ (Transformation|GetActorLocation _array_element) (* (* (Variables|/Game/Asteroids/Blueprints/Asteroid.Asteroid_C|GetMoveVector _array_element) DeltaTime) (Variables|/Game/Asteroids/Blueprints/Asteroid.Asteroid_C|GetMoveSpeed _array_element))) false false)
        (Class|OffScreenUtil|UpdateActorLocationwhenOffScreen _array_element)))))

(fn CheckforDestroyedAsteroids
  (Utilities|Array|Clear (Variables|Default|GetTempAsteroids))
  (for _array_element (Variables|Default|GetAsteroids)
    (Utilities|IsValid _array_element
      (:Is%20Valid
        (Variables|Default|SetCurrentAsteroid _array_element)
        (if (Utilities|Enum|Equal(Enum) (Variables|/Game/Asteroids/Blueprints/Asteroid.Asteroid_C|GetStatus _array_element) "NewEnumerator1")
          (Variables|Default|SetCurrentAsteroidPos (Transformation|GetActorLocation (Variables|Default|GetCurrentAsteroid)))
          (switch Utilities|FlowControl|Switch|SwitchonSize (Variables|/Game/Asteroids/Blueprints/Asteroid.Asteroid_C|GetSize (Variables|Default|GetCurrentAsteroid))
            (:NewEnumerator0
              (Variables|Default|SetSize "NewEnumerator1")
              (Actor|DestroyActor (Variables|Default|GetCurrentAsteroid) :!label _label)
              (for _index (range 0 2)
                (Variables|Default|SetStartSide (Utilities|Enum|ByteToEnumStartSide (Math|Conversions|ToByte(Integer) (Math|Random|RandomInteger 3))))
                (bind _createdasteroid (CallFunction|CreateAsteroid (Variables|Default|GetSize) (Math|Vector|MakeVector (Math|Random|RandomFloatinRange -1.0 1.0) (Math|Random|RandomFloatinRange -1.0 1.0) 0.0) (Variables|Default|GetCurrentAsteroidPos)))
                (Utilities|Array|Add (Variables|Default|GetAsteroids) _createdasteroid)
                (Utilities|Array|Add (Variables|Default|GetTempAsteroids) (Variables|Default|GetCurrentAsteroid))))
            (:NewEnumerator1
              (Variables|Default|SetSize "NewEnumerator2")
              (goto _label))
            (:NewEnumerator2
              (Actor|DestroyActor (Variables|Default|GetCurrentAsteroid))))))))
  (for _array_element_2 (Variables|Default|GetTempAsteroids)
    (Utilities|Array|RemoveItem (Variables|Default|GetAsteroids) _array_element_2)))

(fn CreateAsteroid
  (params (Size :type Size%20Enum :default "NewEnumerator0") (Direction :type Vector) (StartPos :type Vector))
  (bind _returnvalue (Game|SpawnActorfromClass "/Game/Asteroids/Blueprints/Asteroid.Asteroid_C" (Math|Transform|MakeTransform (Math|Vector|MakeVector (.x StartPos) (.y StartPos) -5.0) "0, 0, 0" "1,1,1") "Undefined" 0 0))
  (bind _asteroid (Default|Initialize _returnvalue Size (Variables|Default|GetStartSide) Direction))
  (return _asteroid))