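; Asteroid actor for an Asteroids game, set up through an Initialize function that takes a size and a starting side.
; Initialize derives MoveVector from the side, pointing along one axis with a random cross-axis drift, then triples the mesh scale for Large.
; Only Left, Right and Top are wired, leaving the negative-Y branch unreachable, and only Large changes scale.
; BeginPlay and Tick are empty, so nothing here applies the movement.
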(event EventTick
  (params (DeltaSeconds :type Float%20%28single-precision%29)))

(event EventBeginPlay)

(fn ConstructionScript)

(fn Initialize
  (params (Size :type Size%20Enum :default "NewEnumerator0") (StartSide :type StartSide%20Enum :default "NewEnumerator0"))
  (Variables|Default|SetSize Size)
  (Variables|Default|SetStartSide StartSide)
  (Variables|Default|SetCoefficient (Math|Random|RandomFloatinRange -1.0 1.0))
  (switch Utilities|FlowControl|Switch|SwitchonStartSide (Variables|Default|GetStartSide)
    (:NewEnumerator0
      (Variables|Default|SetMoveVector (Math|Vector|MakeVector 1.0 (Variables|Default|GetCoefficient) 0.0)))
    (:NewEnumerator1
      (Variables|Default|SetMoveVector (Math|Vector|MakeVector -1.0 (Variables|Default|GetCoefficient) 0.0)))
    (:NewEnumerator2
      (Variables|Default|SetMoveVector (Math|Vector|MakeVector (Variables|Default|GetCoefficient) 1.0 0.0))))
  (switch Utilities|FlowControl|Switch|SwitchonSize (Variables|Default|GetSize)
    (:NewEnumerator0
      (Transformation|SetWorldScale3D (Variables|Default|GetAsteroid) "3.000000,3.000000,3.000000"))))